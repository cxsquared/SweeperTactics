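; Board is an Actor Blueprint that stores a two-dimensional grid of tiles and looks them up by coordinate.
; GetTile reads the nested Tiles array by row Y and column X.
; Out-of-range coordinates only print a warning, and the lookup still runs afterwards.
; The event graph and construction script hold no logic.
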(fn `GetTile`
  (params (y :type Integer) (x :type Integer))
  (returns (Tile :type "/Game/Structs/Tile Structure"))
  (if (or (< y 0) (< x 0) (>= y (`self.Height`)) (>= x (`self.Width`)))
    (`KismetSystemLibrary.PrintText` "Invalid X/Y when getting tile." true true (struct :`R` 1.0 :`B` 0.149952 :`A` 1.0) 5.0))
  (return (`|GetArrayItem` (`.Tiles_3_3502F1B34B18B895EEBEA6BC78BFF974` (break `/Game/Structs/TileArray` (`|GetArrayItem` (`self.Tiles`) y))) x)))

(fn `UserConstructionScript`)